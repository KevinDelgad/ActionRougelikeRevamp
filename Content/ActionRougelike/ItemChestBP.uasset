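; Treasure chest actor that a pawn interacts with, opening only if that pawn holds the required keycard gameplay tag.
; Interact checks the instigator's action component active tags, then a FlipFlop alternates playing and reversing a lid timeline that drives the lid's pitch.
; A finished timeline activates the gold burst effect, while a missing tag prints a red debug message.
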(event `SGameplayInterface.Interact`
  (params (InstigatorPawn :type "Pawn Object Reference"))
  (if (`BlueprintGameplayTagLibrary.HasTag` (`SActionComponent.ActiveGameplayTags` (`self.GetComponentByClass` InstigatorPawn "/Script/ActionRougelikeRe.SActionComponent")) (`self.Required Keycard`) true)
    (`/Engine/EditorBlueprintResources/StandardMacros.FlipFlop`
      (:`A`
        (bind (_direction _pitch) (`Timeline|AnimateLid` :!label _label)
          (:`Update`
            (`SceneComponent.K2_SetRelativeRotation` (`self.LidMesh`) (`KismetMathLibrary.MakeRotator` 0.0 _pitch) false false))
          (:`Finished`
            (`ActorComponent.Activate` (`self.Gold Burst`) false))))
      (:`B`
        (goto _label :!via `Reverse`)))
    (else
      (`KismetSystemLibrary.PrintString` (`KismetStringLibrary.Concat_StrStr` "Missing Tag: " (`BlueprintGameplayTagLibrary.GetDebugStringFromGameplayTag` (`self.Required Keycard`))) true true (struct :`R` 1.0 :`G` 0.030305 :`A` 1.0)))))

(fn `UserConstructionScript`)